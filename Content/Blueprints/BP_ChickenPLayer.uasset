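; Player chicken Blueprint that spends collected corn to lay eggs and plays an idle chicken sound on BeginPlay.
; Fire checks three Corns tiers, spawning a BP_Egg at EggSpawnPoint and launching it with a fixed impulse.
; Each tier deducts its corn cost and sets PointsToAdd, with higher tiers swapping the egg material, up to gold.
; A and D snap the mesh rotation to face opposite sides.
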(event `InputAction|Fire`
  (params (Key :type "Key Structure"))
  (:`Pressed`
    (`|ExecutionSequence`
      (:`then_0`
        (if (>= (`self.Corns`) 10)
          (if (<= (`self.Corns`) 14)
            (bind _returnvalue (`|SpawnActorFromClass` "/Game/Blueprints/BP_Egg.BP_Egg_C" (`SceneComponent.K2_GetComponentToWorld` (`self.EggSpawnPoint`)) "Undefined" "OverrideRootScale" null null))
            (`PrimitiveComponent.AddImpulse` (`/Game/Blueprints/BP_Egg.StaticMesh` _returnvalue) (0.0 250.0 850.0) "None" false)
            (set `self.Corns` (- (`self.Corns`) 10))
            (set `self.PointsToAdd` 5))))
      (:`then_1`
        (if (>= (`self.Corns`) 15)
          (if (<= (`self.Corns`) 19)
            (bind _returnvalue_2 (`|SpawnActorFromClass` "/Game/Blueprints/BP_Egg.BP_Egg_C" (`SceneComponent.K2_GetComponentToWorld` (`self.EggSpawnPoint`)) "Undefined" "OverrideRootScale" null null))
            (bind _staticmesh (`/Game/Blueprints/BP_Egg.StaticMesh` _returnvalue_2))
            (`PrimitiveComponent.SetMaterial` _staticmesh 0 "/Game/Materials/M_Egg_Inst_Inst.M_Egg_Inst_Inst")
            (`PrimitiveComponent.AddImpulse` _staticmesh (0.0 250.0 850.0) "None" false)
            (set `self.Corns` (- (`self.Corns`) 15))
            (set `self.PointsToAdd` 10))))
      (:`then_2`
        (if (>= (`self.Corns`) 20)
          (bind _returnvalue_3 (`|SpawnActorFromClass` "/Game/Blueprints/BP_Egg.BP_Egg_C" (`SceneComponent.K2_GetComponentToWorld` (`self.EggSpawnPoint`)) "Undefined" "OverrideRootScale" null null))
          (bind _staticmesh_2 (`/Game/Blueprints/BP_Egg.StaticMesh` _returnvalue_3))
          (`PrimitiveComponent.SetMaterial` _staticmesh_2 0 "/Game/StarterContent/Materials/M_Metal_Gold.M_Metal_Gold")
          (`PrimitiveComponent.AddImpulse` _staticmesh_2 (0.0 250.0 850.0) "None" false)
          (set `self.Corns` (- (`self.Corns`) 20))
          (set `self.PointsToAdd` 15))))))

(event `self.ReceiveBeginPlay`
  (`GameplayStatics.PlaySound2D` "/Game/Sounds/ChickenIdle_Cue.ChickenIdle_Cue" 1.0 1.0 0.0 null null))

(event `Key|A`
  (params (Key :type "Key Structure"))
  (:`Pressed`
    (`SceneComponent.K2_SetRelativeRotation` (`self.Mesh`) (struct :`Yaw` 90.0) false false)))

(event `Key|D`
  (params (Key :type "Key Structure"))
  (:`Pressed`
    (`SceneComponent.K2_SetRelativeRotation` (`self.Mesh`) (struct :`Yaw` -90.0) false false)))

(fn `UserConstructionScript`)