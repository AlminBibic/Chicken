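; Game mode that runs a minutes-and-seconds countdown and ends the game when it reaches zero, also capping frame rate at 60 on BeginPlay.
; Tick feeds a one-second Delay to step the timer about once per second.
; At zero it shows WBP_GameOver and the mouse cursor, disables pawn input and sets IsgameOver.
; An unconnected count-up version of the timer remains in the graph.
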(event `self.ReceiveBeginPlay`
  (bind _returnvalue (`GameUserSettings.GetGameUserSettings`))
  (`GameUserSettings.SetFrameRateLimit` _returnvalue 60.0))

(event `self.ReceiveTick`
  (params (DeltaSeconds :type "Float (single-precision)"))
  (bind _returnvalue (`GameplayStatics.GetPlayerController` 0))
  (`KismetSystemLibrary.Delay` 1.0)
  (set `self.Seconds` (- (`self.Seconds`) 1))
  (if (< (`self.Seconds`) 0)
    (set `self.Minutes` (- (`self.Minutes`) 1))
    (set `self.Seconds` 59))
  (if (== (`self.Seconds`) 0)
    (if (== (`self.Minutes`) 0)
      (`KismetSystemLibrary.PrintString` "Game Over")
      (bind _returnvalue_2 (`|CreateWidget` "/Game/Blueprints/WBP_GameOver.WBP_GameOver_C"))
      (`UserWidget.AddToViewport` _returnvalue_2 0)
      (set `PlayerController.bShowMouseCursor` true _returnvalue)
      (`self.DisableInput` (`GameplayStatics.GetPlayerPawn` 0) _returnvalue)
      (set `self.IsgameOver` true))))

(fn `UserConstructionScript`)